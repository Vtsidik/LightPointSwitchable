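; Point light Blueprint that a control button switches on and off.
; On BeginPlay it binds its toggle event to the ControlButton's OnPressed dispatcher.
; The toggle checks the TurnedON flag and calls TurnOn or TurnOff, which set the light's visibility and return the new state to store in that flag.
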(event `self.ReceiveBeginPlay`
  (add `/Game/Blueprints/BP_BaseInteractible.OnPressed` (`self.ControlButton`) (delegate `TurnOn/Off`)))

(event `TurnOn/Off`
  (if (`self.TurnedON?`)
    (bind _off (`self.TurnOff`))
    (set `self.TurnedON?` _off)
    (else
      (bind _on (`self.TurnOn`))
      (set `self.TurnedON?` _on))))

(fn `TurnOff`
  (returns (Off :type Boolean))
  (`SceneComponent.SetVisibility` (`self.PointLight`) false false)
  (return false))

(fn `TurnOn`
  (returns (On :type Boolean))
  (`SceneComponent.SetVisibility` (`self.PointLight`) true false)
  (return true))

(fn `UserConstructionScript`)